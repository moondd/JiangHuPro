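; Character Blueprint with modular body and pants meshes and RPG stats, initialized from a per-character save or randomized when none exists.
; On BeginPlay it loads or rolls attributes and part IDs, applies data table meshes with randomly tinted dynamic materials, then derives health, mana, damage, resistance and penetration.
; The construction script links both parts to the main mesh via master pose and fills skill slots from a data table.
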(event `self.ReceiveBeginPlay`
  (`self.LoadData`)
  (`self.SetMesh`)
  (`self.SetProperty `))

(fn `LoadData`
  (bind _returnvalue (`KismetStringLibrary.BuildString_Name` "DD/" (`KismetSystemLibrary.GetDisplayName` self)))
  (bind _returnvalue_2 (`GameplayStatics.DoesSaveGameExist` _returnvalue))
  (if _returnvalue_2
    (bind _returnvalue_3 (`GameplayStatics.LoadGameFromSlot` _returnvalue))
    (bind _ascharacter_save_data (cast `/Game/SaveData/CharacterSaveData` _returnvalue_3))
    (`|ExecutionSequence`
      (:`then_0`
        (set `self.CurrMana` (`/Game/SaveData/CharacterSaveData.CurrMana` _ascharacter_save_data)))
      (:`then_1`
        (set `self.CurrHealth` (`/Game/SaveData/CharacterSaveData.CurrHealth` _ascharacter_save_data)))
      (:`then_2`
        (set `self.CON` (`/Game/SaveData/CharacterSaveData.CON` _ascharacter_save_data)))
      (:`then_3`
        (set `self.STR` (`/Game/SaveData/CharacterSaveData.STR` _ascharacter_save_data)))
      (:`then_4`
        (set `self.DEF` (`/Game/SaveData/CharacterSaveData.DEF` _ascharacter_save_data)))
      (:`then_5`
        (set `self.INT` (`/Game/SaveData/CharacterSaveData.INT` _ascharacter_save_data)))
      (:`then_6`
        (set `self.Health` (`/Game/SaveData/CharacterSaveData.Health` _ascharacter_save_data)))
      (:`then_7`
        (set `self.Damage` (`/Game/SaveData/CharacterSaveData.Damage` _ascharacter_save_data)))
      (:`then_8`
        (set `self.Defense` (`/Game/SaveData/CharacterSaveData.Defense` _ascharacter_save_data)))
      (:`then_9`
        (set `self.Mana` (`/Game/SaveData/CharacterSaveData.Mana` _ascharacter_save_data)))
      (:`then_10`
        (set `self.BodyID` (`/Game/SaveData/CharacterSaveData.BodyID` _ascharacter_save_data)))
      (:`then_11`
        (set `self.PantsID` (`/Game/SaveData/CharacterSaveData.PantsID` _ascharacter_save_data))))
    (else
      (`|ExecutionSequence`
        (:`then_0`
          (set `self.CON` (`KismetMathLibrary.RandomInteger` 100)))
        (:`then_1`
          (set `self.STR` (`KismetMathLibrary.RandomInteger` 100)))
        (:`then_2`
          (set `self.DEF` (`KismetMathLibrary.RandomInteger` 100)))
        (:`then_3`
          (set `self.INT` (`KismetMathLibrary.RandomInteger` 100)))
        (:`then_4`
          (set `self.Health` (`KismetMathLibrary.RandomInteger` 100)))
        (:`then_5`
          (set `self.Damage` (`KismetMathLibrary.RandomInteger` 100)))
        (:`then_6`
          (set `self.Defense` (`KismetMathLibrary.RandomInteger` 100)))
        (:`then_7`
          (set `self.Mana` (`KismetMathLibrary.RandomInteger` 100)))
        (:`then_8`
          (set `self.BodyID` (`KismetStringLibrary.Conv_StringToName` (`KismetStringLibrary.Conv_IntToString` (`KismetMathLibrary.RandomIntegerInRange` 1 2)))))
        (:`then_9`
          (set `self.PantsID` (`KismetStringLibrary.Conv_StringToName` (`KismetStringLibrary.Conv_IntToString` (`KismetMathLibrary.RandomIntegerInRange` 1 2)))))))))

(fn `SetMesh`
  (bind _body (`self.Body`))
  (bind _pants (`self.Pants`))
  (bind _returnvalue (`PrimitiveComponent.GetMaterial` _body 0))
  (bind _returnvalue_2 (`PrimitiveComponent.GetMaterial` _pants 0))
  (`|ExecutionSequence`
    (:`then_0`
      (bind _returnvalue_3 (`|GetDataTableRow` "/Game/SaveData/BodyDataTable.BodyDataTable" (`self.BodyID`))
        (:`then`
          (`SkinnedMeshComponent.SetSkinnedAssetAndUpdate` _body (`.Mesh_5_D3279C78497200213C21409F8E49A76C` (break `/Game/SaveData/EqipStruct` _returnvalue_3)) true)
          (bind _returnvalue_4 (`KismetMaterialLibrary.CreateDynamicMaterialInstance` _returnvalue _returnvalue))
          (`PrimitiveComponent.SetMaterial` (`self.Body`) 0 _returnvalue_4)
          (`MaterialInstanceDynamic.SetVectorParameterValue` _returnvalue_4 "ClothColor" (`KismetMathLibrary.MakeColor` (`KismetMathLibrary.RandomFloatInRange` 0.01 0.2) (`KismetMathLibrary.RandomFloatInRange` 0.01 0.2) (`KismetMathLibrary.RandomFloatInRange` 0.01 0.2))))))
    (:`then_1`
      (bind _returnvalue_5 (`|GetDataTableRow` "/Game/SaveData/PantsDataTable.PantsDataTable" (`self.PantsID`))
        (:`then`
          (`SkinnedMeshComponent.SetSkinnedAssetAndUpdate` _pants (`.Mesh_5_D3279C78497200213C21409F8E49A76C` (break `/Game/SaveData/EqipStruct` _returnvalue_5)) true)
          (bind _returnvalue_6 (`KismetMaterialLibrary.CreateDynamicMaterialInstance` _returnvalue_2 _returnvalue_2))
          (`PrimitiveComponent.SetMaterial` _pants 0 _returnvalue_6)
          (`MaterialInstanceDynamic.SetVectorParameterValue` _returnvalue_6 "ClothColor" (`KismetMathLibrary.MakeColor` (`KismetMathLibrary.RandomFloatInRange` 0.01 0.2) (`KismetMathLibrary.RandomFloatInRange` 0.01 0.2) (`KismetMathLibrary.RandomFloatInRange` 0.01 0.2))))))))

(fn `SetProperty `
  (`|ExecutionSequence`
    (:`then_0`
      (set `self.Add_Health` (+ 6.0 (* (* (`self.CON`) 0.01) 3.0))))
    (:`then_1`
      (set `self.Add_Damage` (+ 1.0 (* (* (`self.STR`) 0.01) 1.0))))
    (:`then_2`
      (set `self.Add_Defense` (+ 10.0 (* (* (`self.DEF`) 0.01) 10.0))))
    (:`then_3`
      (set `self.Add_IntDamage` (+ 10.0 (* (* (`self.INT`) 0.01) 10.0)))))
  (`|ExecutionSequence`
    (:`then_0`
      (set `self.MaxHealth` (+ (* (`self.Health`) (`self.Add_Health`)) 60.0)))
    (:`then_1`
      (set `self.MaxMana` (+ (* (* (`self.Mana`) (`self.Add_Damage`)) 6.0) 60.0)))
    (:`then_2`
      (set `self.CurrDamage` (+ (* (`self.Damage`) (`self.Add_Damage`)) 10.0)))
    (:`then_3`
      (set `self.CurrResistance` (- 1.0 (/ 100.0 (+ 100.0 (* (`self.Defense`) (`self.Add_Defense`)))))))
    (:`then_4`
      (set `self.CurrPenetrate` (- 1.0 (/ 100.0 (+ 100.0 (* (`self.Mana`) (`self.Add_IntDamage`)))))))))

(fn `SetSkillsStruct`
  (params (SkillID :type Integer))
  (bind _returnvalue (`|GetDataTableRow` "/Game/MyCharacter/SkillsDataTable.SkillsDataTable" "1")
    (:`then`
      (set `self.SkillsStruct` (`|MakeArray` _returnvalue _returnvalue (struct) (struct) (struct) (struct))))))

(fn `UserConstructionScript`
  (bind _mesh (`self.Mesh`))
  (`SkinnedMeshComponent.SetLeaderPoseComponent` (`self.Body`) _mesh)
  (`SkinnedMeshComponent.SetLeaderPoseComponent` (`self.Pants`) _mesh)
  (`self.SetSkillsStruct` 0))