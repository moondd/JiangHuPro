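; Player controller that caches the possessed CharacterBP_Player, creates the main HUD and dialogue widgets, and shows the mouse cursor.
; Axis input drives yaw-relative movement and camera look, while action input sets attack, block, jump and skill flags on the character and toggles its equip state.
; Every tick it runs a short debug-drawn camera-channel trace from the spring arm along the camera's forward, only printing the hit actor as a dialogue-target probe.
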(event `self.ReceiveBeginPlay`
  (`self.InitializePlayer`)
  (bind _returnvalue (`|CreateWidget` "/Game/MyCharacter/Blueprints/MyHUD.MyHUD_C"))
  (bind _output_get (set `self.MHUD` _returnvalue))
  (`UserWidget.AddToViewport` _output_get 0)
  (bind _returnvalue_2 (`|CreateWidget` "/Game/MyCharacter/DialogSystem/DialogueBlueprint.DialogueBlueprint_C"))
  (bind _output_get_2 (set `self.DialogHUD` _returnvalue_2))
  (`UserWidget.AddToViewport` _output_get_2 0)
  (set `self.bShowMouseCursor` true))

(event `self.ReceiveTick`
  (params (DeltaSeconds :type "Float (single-precision)"))
  (`self.FindDialogueTarget`))

(event `InputAction|Block`
  (params (Key :type "Key Structure" :default "AnyKey"))
  (bind _characterref (`self.CharacterRef`))
  ;[1 1 1] 防御
  (:`Pressed`
    (set `/Game/MyCharacter/Blueprints/CharacterBP_Action.DoBlock?` true _characterref))
  (:`Released`
    (set `/Game/MyCharacter/Blueprints/CharacterBP_Action.DoBlock?` false _characterref)))

(event `InputAxis|MoveFoward`
  (params (AxisValue :type "Float (single-precision)"))
  (bind _characterref (`self.CharacterRef`))
  ;[1 1 1] 移动
  (`/Engine/EditorBlueprintResources/StandardMacros.IsValid` _characterref
    (:`Is Valid`
      (`Pawn.AddMovementInput` _characterref (`KismetMathLibrary.GetForwardVector` (`KismetMathLibrary.MakeRotator` 0.0 0.0 (.yaw (`self.GetControlRotation`)))) AxisValue false))))

(event `InputAction|Attack`
  (params (Key :type "Key Structure" :default "AnyKey"))
  (bind _characterref (`self.CharacterRef`))
  ;[1 1 1] 攻击
  (:`Pressed`
    (set `/Game/MyCharacter/Blueprints/CharacterBP_Action.DoAttack?` true _characterref))
  (:`Released`
    (set `/Game/MyCharacter/Blueprints/CharacterBP_Action.DoAttack?` false _characterref)))

(event `InputAxis|MoveRight`
  (params (AxisValue :type "Float (single-precision)"))
  (bind _characterref (`self.CharacterRef`))
  ;[1 1 1] 移动
  (`/Engine/EditorBlueprintResources/StandardMacros.IsValid` _characterref
    (:`Is Valid`
      (`Pawn.AddMovementInput` _characterref (`KismetMathLibrary.GetRightVector` (`KismetMathLibrary.MakeRotator` 0.0 0.0 (.yaw (`self.GetControlRotation`)))) AxisValue false))))

(event `InputAction|IdleState`
  (params (Key :type "Key Structure" :default "AnyKey"))
  (bind _characterref (`self.CharacterRef`))
  ;[1 1 1] 和平/战斗
  (:`Pressed`
    (if (`|EnumEquality` (`/Game/MyCharacter/Blueprints/CharacterBP_Action.EqipState` _characterref) "NewEnumerator2")
      (set `/Game/MyCharacter/Blueprints/CharacterBP_Action.EqipState` "NewEnumerator1" _characterref)
      (else
        (set `/Game/MyCharacter/Blueprints/CharacterBP_Action.EqipState` "NewEnumerator2" _characterref)))))

(event `InputAxis|Turn`
  (params (AxisValue :type "Float (single-precision)"))
  (bind _characterref (`self.CharacterRef`))
  ;[1 1 1] 视角
  (`/Engine/EditorBlueprintResources/StandardMacros.IsValid` _characterref
    (:`Is Valid`
      (`Pawn.AddControllerYawInput` _characterref AxisValue))))

(event `InputAxis|LookUp`
  (params (AxisValue :type "Float (single-precision)"))
  (bind _characterref (`self.CharacterRef`))
  ;[1 1 1] 视角
  (`/Engine/EditorBlueprintResources/StandardMacros.IsValid` _characterref
    (:`Is Valid`
      (`Pawn.AddControllerPitchInput` _characterref AxisValue))))

(event `InputAction|Skill0`
  (params (Key :type "Key Structure" :default "AnyKey"))
  (bind _characterref (`self.CharacterRef`))
  (:`Pressed`
    (set `/Game/MyCharacter/Blueprints/CharacterBP_Action.DoSkill` "NewEnumerator1" _characterref))
  (:`Released`
    (set `/Game/MyCharacter/Blueprints/CharacterBP_Action.DoSkill` "NewEnumerator0" _characterref)))

(event `InputAction|Jump`
  (params (Key :type "Key Structure" :default "AnyKey"))
  (bind _characterref (`self.CharacterRef`))
  ;[1 1 1] InputJump
  (:`Pressed`
    (set `/Game/MyCharacter/Blueprints/CharacterBP_Action.DoJump?` true _characterref))
  (:`Released`
    (set `/Game/MyCharacter/Blueprints/CharacterBP_Action.DoJump?` false _characterref)))

(fn `FindDialogueTarget`
  (bind _characterref (`self.CharacterRef`))
  (bind _returnvalue (`SceneComponent.K2_GetComponentLocation` (`/Game/MyCharacter/Blueprints/CharacterBP_Player.SpringArm` _characterref)))
  (bind _outhit (`KismetSystemLibrary.LineTraceSingle` _returnvalue (+ _returnvalue (* (`SceneComponent.GetForwardVector` (`/Game/MyCharacter/Blueprints/CharacterBP_Player.Camera` _characterref)) 100.0)) "TraceTypeQuery2" false (`|MakeArray` (`GameplayStatics.GetPlayerPawn` 0) :!type "Actor Object Reference") "ForDuration"))
  (`KismetSystemLibrary.PrintString` (`KismetSystemLibrary.GetDisplayName` (`.HitActor` (`GameplayStatics.BreakHitResult` _outhit)))))

(fn `InitializePlayer`
  (bind _ascharacter_bp_player (cast `/Game/MyCharacter/Blueprints/CharacterBP_Player` (`self.K2_GetPawn`)))
  (set `self.CharacterRef` _ascharacter_bp_player))

(fn `UserConstructionScript`)