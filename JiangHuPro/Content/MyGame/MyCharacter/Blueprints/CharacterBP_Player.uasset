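; Player character Blueprint that defers BeginPlay, Tick and construction to its parent and holds a test-like, unfinished save hook.
; Releasing Left Alt creates a CharacterSaveData object and copies only Health (气血) into it, without writing it to disk.
; A disconnected sequence would copy stats and body/pants IDs, saving to a slot built from "DD/" and the display name, but never runs.
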(event `self.ReceiveBeginPlay`
  (`parent.ReceiveBeginPlay`))

(event `self.ReceiveTick`
  (params (DeltaSeconds :type "Float (single-precision)"))
  (`parent.ReceiveTick` 0.0))

(event `Key|LeftAlt`
  (params (Key :type "Key Structure" :default "AnyKey"))
  (:`Released`
    (bind _returnvalue (`GameplayStatics.CreateSaveGameObject` "/Game/MyGame/SaveData/CharacterSaveData.CharacterSaveData_C"))
    (bind _ascharacter_save_data (cast `/Game/MyGame/SaveData/CharacterSaveData` _returnvalue))
    (set `/Game/MyGame/SaveData/CharacterSaveData.Health` (`self.气血`) _ascharacter_save_data)))

(fn `UserConstructionScript`
  (`parent.UserConstructionScript`))