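; Modular RPG character Blueprint with wuxia-style attributes, a morality alignment and a skill list.
; On BeginPlay it loads attributes and outfit IDs from a per-character save, or randomizes attributes with default outfit IDs, then derives combat stats through growth factors.
; Body and Pants follow the main mesh via master pose, taking meshes from DataTables and random cloth tints through dynamic materials.
; It also rolls alignment, seeds skills at construction and defines an uncalled random-name generator.
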(event `self.ReceiveBeginPlay`
  (`self.LoadData`)
  (`self.SetMesh`)
  (`self.SetProperty `)
  (`self.设置善恶值`))

(fn `LoadData`
  (bind _returnvalue (`KismetStringLibrary.BuildString_Name` "DD/" (`KismetSystemLibrary.GetDisplayName` self)))
  (bind _returnvalue_2 (`GameplayStatics.DoesSaveGameExist` _returnvalue))
  (if _returnvalue_2
    (bind _returnvalue_3 (`GameplayStatics.LoadGameFromSlot` _returnvalue))
    (bind _ascharacter_save_data (cast `/Game/MyGame/GameData/CharacterSaveData` _returnvalue_3))
    (`|ExecutionSequence`
      (:`then_0`
        (set `self.当前内力` (`/Game/MyGame/GameData/CharacterSaveData.CurrMana` _ascharacter_save_data)))
      (:`then_1`
        (set `self.当前气血` (`/Game/MyGame/GameData/CharacterSaveData.CurrHealth` _ascharacter_save_data)))
      (:`then_2`
        (set `self.根骨` (`/Game/MyGame/GameData/CharacterSaveData.CON` _ascharacter_save_data)))
      (:`then_3`
        (set `self.臂力` (`/Game/MyGame/GameData/CharacterSaveData.STR` _ascharacter_save_data)))
      (:`then_4`
        (set `self.定力` (`/Game/MyGame/GameData/CharacterSaveData.DEF` _ascharacter_save_data)))
      (:`then_5`
        (set `self.内功` (`/Game/MyGame/GameData/CharacterSaveData.INT` _ascharacter_save_data)))
      (:`then_6`
        (set `self.气血` (`/Game/MyGame/GameData/CharacterSaveData.Health` _ascharacter_save_data)))
      (:`then_7`
        (set `self.伤害` (`/Game/MyGame/GameData/CharacterSaveData.Damage` _ascharacter_save_data)))
      (:`then_8`
        (set `self.防御` (`/Game/MyGame/GameData/CharacterSaveData.Defense` _ascharacter_save_data)))
      (:`then_9`
        (set `self.内力` (`/Game/MyGame/GameData/CharacterSaveData.Mana` _ascharacter_save_data)))
      (:`then_10`
        (set `self.BodyID` (`/Game/MyGame/GameData/CharacterSaveData.BodyID` _ascharacter_save_data)))
      (:`then_11`
        (set `self.PantsID` (`/Game/MyGame/GameData/CharacterSaveData.PantsID` _ascharacter_save_data))))
    (else
      (`|ExecutionSequence`
        (:`then_0`
          (set `self.根骨` (`KismetMathLibrary.RandomInteger` 100)))
        (:`then_1`
          (set `self.臂力` (`KismetMathLibrary.RandomInteger` 100)))
        (:`then_2`
          (set `self.定力` (`KismetMathLibrary.RandomInteger` 100)))
        (:`then_3`
          (set `self.内功` (`KismetMathLibrary.RandomInteger` 100)))
        (:`then_4`
          (set `self.气血` (`KismetMathLibrary.RandomInteger` 100)))
        (:`then_5`
          (set `self.伤害` (`KismetMathLibrary.RandomInteger` 100)))
        (:`then_6`
          (set `self.防御` (`KismetMathLibrary.RandomInteger` 100)))
        (:`then_7`
          (set `self.内力` (`KismetMathLibrary.RandomInteger` 100)))
        (:`then_8`
          (set `self.BodyID` (`KismetStringLibrary.Conv_StringToName` (`KismetStringLibrary.Conv_IntToString` 2))))
        (:`then_9`
          (set `self.PantsID` (`KismetStringLibrary.Conv_StringToName` (`KismetStringLibrary.Conv_IntToString` 2))))))))

(fn `SetMesh`
  (bind _body (`self.Body`))
  (bind _pants (`self.Pants`))
  (bind _returnvalue (`PrimitiveComponent.GetMaterial` _body 0))
  (bind _returnvalue_2 (`PrimitiveComponent.GetMaterial` _pants 0))
  (`|ExecutionSequence`
    (:`then_0`
      (bind _returnvalue_3 (`|GetDataTableRow` "/Game/MyGame/GameData/BodyDataTable.BodyDataTable" (`self.BodyID`))
        (:`then`
          (`SkinnedMeshComponent.SetSkinnedAssetAndUpdate` _body (`.Mesh_5_D3279C78497200213C21409F8E49A76C` (break `/Game/MyGame/GameData/EqipStruct` _returnvalue_3)) true)
          (bind _returnvalue_4 (`KismetMaterialLibrary.CreateDynamicMaterialInstance` _returnvalue _returnvalue))
          (`PrimitiveComponent.SetMaterial` (`self.Body`) 0 _returnvalue_4)
          (`MaterialInstanceDynamic.SetVectorParameterValue` _returnvalue_4 "ClothColor" (`KismetMathLibrary.MakeColor` (`KismetMathLibrary.RandomFloatInRange` 0.01 0.2) (`KismetMathLibrary.RandomFloatInRange` 0.01 0.2) (`KismetMathLibrary.RandomFloatInRange` 0.01 0.2))))))
    (:`then_1`
      (bind _returnvalue_5 (`|GetDataTableRow` "/Game/MyGame/GameData/PantsDataTable.PantsDataTable" (`self.PantsID`))
        (:`then`
          (`SkinnedMeshComponent.SetSkinnedAssetAndUpdate` _pants (`.Mesh_5_D3279C78497200213C21409F8E49A76C` (break `/Game/MyGame/GameData/EqipStruct` _returnvalue_5)) true)
          (bind _returnvalue_6 (`KismetMaterialLibrary.CreateDynamicMaterialInstance` _returnvalue_2 _returnvalue_2))
          (`PrimitiveComponent.SetMaterial` _pants 0 _returnvalue_6)
          (`MaterialInstanceDynamic.SetVectorParameterValue` _returnvalue_6 "ClothColor" (`KismetMathLibrary.MakeColor` (`KismetMathLibrary.RandomFloatInRange` 0.01 0.2) (`KismetMathLibrary.RandomFloatInRange` 0.01 0.2) (`KismetMathLibrary.RandomFloatInRange` 0.01 0.2))))))))

(fn `SetProperty `
  (`|ExecutionSequence`
    (:`then_0`
      (set `self.气血成长` (+ 6.0 (* (* (`self.根骨`) 0.01) 3.0))))
    (:`then_1`
      (set `self.伤害成长` (+ 1.0 (* (* (`self.臂力`) 0.01) 1.0))))
    (:`then_2`
      (set `self.防御成长` (+ 10.0 (* (* (`self.定力`) 0.01) 10.0))))
    (:`then_3`
      (set `self.内力成长` (+ 10.0 (* (* (`self.内功`) 0.01) 10.0)))))
  (`|ExecutionSequence`
    (:`then_0`
      (set `self.最大气血` (+ (* (`self.气血`) (`self.气血成长`)) 60.0)))
    (:`then_1`
      (set `self.最大内力` (+ (* (* (`self.内力`) (`self.伤害成长`)) 6.0) 60.0)))
    (:`then_2`
      (set `self.伤害值` (+ (* (`self.伤害`) (`self.伤害成长`)) 10.0)))
    (:`then_3`
      (set `self.伤害吸收` (- 1.0 (/ 100.0 (+ 100.0 (* (`self.防御`) (`self.防御成长`)))))))
    (:`then_4`
      (set `self.伤害穿透` (- 1.0 (/ 100.0 (+ 100.0 (* (`self.内力`) (`self.内力成长`)))))))))

(fn `SetSkillsStruct`
  (params (SkillID :type Integer))
  (bind _returnvalue (`|GetDataTableRow` "/Game/MyGame/MyCharacter/SkillsDataTable.SkillsDataTable" "1")
    (:`then`
      (set `self.当前技能列表` (`|MakeArray` _returnvalue _returnvalue (struct) (struct) (struct) (struct))))))

(fn `UserConstructionScript`
  (bind _mesh (`self.Mesh`))
  (`SkinnedMeshComponent.SetLeaderPoseComponent` (`self.Body`) _mesh)
  (`SkinnedMeshComponent.SetLeaderPoseComponent` (`self.Pants`) _mesh)
  (`self.SetSkillsStruct` 0))

(fn `设置善恶值`
  (bind _output_get (set `self.善恶值` (`KismetMathLibrary.RandomIntegerInRange` -125 125)))
  (if (<= _output_get -75)
    (set `self.性向` "NewEnumerator0")
    (elif (<= _output_get -25)
      (set `self.性向` "NewEnumerator1")
      (elif (<= _output_get 25)
        (set `self.性向` "NewEnumerator2")
        (elif (<= _output_get 75)
          (set `self.性向` "NewEnumerator3")
          (else
            (set `self.性向` "NewEnumerator4"))))))
  (return))

(fn `随机创建姓名`
  (bind _outrownames (`DataTableFunctionLibrary.GetDataTableRowNames` "/Game/MyGame/GameData/Surname.Surname"))
  (bind _returnvalue (`|GetDataTableRow` "/Game/MyGame/GameData/Surname.Surname" (`KismetStringLibrary.Conv_StringToName` (`KismetStringLibrary.Conv_IntToString` (`KismetMathLibrary.RandomIntegerInRange` 1 (`KismetArrayLibrary.Array_LastIndex` _outrownames)))))
    (:`then`
      (set `self.姓` (`.Name_4_FA1D0D374C5D65444B104588C40FC9A7` (break `/Game/MyGame/GameData/FullNameStruct` _returnvalue)))
      (bind _outrownames_2 (`DataTableFunctionLibrary.GetDataTableRowNames` "/Game/MyGame/GameData/MaleName.MaleName"))
      (bind _returnvalue_2 (`|GetDataTableRow` "/Game/MyGame/GameData/MaleName.MaleName" (`KismetStringLibrary.Conv_StringToName` (`KismetStringLibrary.Conv_IntToString` (`KismetMathLibrary.RandomIntegerInRange` 1 (`KismetArrayLibrary.Array_LastIndex` _outrownames_2)))))
        (:`then`
          (set `self.名` (`.Name_4_FA1D0D374C5D65444B104588C40FC9A7` (break `/Game/MyGame/GameData/FullNameStruct` _returnvalue_2))))))))