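; Player controller that turns input into movement, camera, combat and interaction commands on the player character.
; A state of normal, dialogue or interacting gates most actions and switches cursor, input mode and HUD, with non-"Map_" levels starting in dialogue.
; A per-tick camera-direction line trace picks AI or objects to interact with; dialogue is signalled through the AI's blackboard.
; Hard-coded keys save, load and advance the save's date.
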(event `self.ReceiveBeginPlay`
  (`self.玩家控制器初始化`)
  (bind _returnvalue (`GameplayStatics.GetCurrentLevelName` true))
  (if (`KismetStringLibrary.EqualEqual_StrStr` (`KismetStringLibrary.Split` _returnvalue "_") "Map")
    (`self.设置玩家控制器状态` "NewEnumerator0")
    (else
      (`self.设置玩家控制器状态` "NewEnumerator1"))))

(event `self.ReceiveTick`
  (params (DeltaSeconds :type "Float (single-precision)"))
  (`self.射线检测互动Actor`))

(event `InputAxis|MoveFoward`
  (params (AxisValue :type "Float (single-precision)"))
  (bind `_玩家角色` (`self.玩家角色`))
  ;[1 1 1] PlayertInput
  ;;[1 1 1] 移动
  (bind _caninput_ (`self.能否进行操作?`))
  (if _caninput_
    (`/Engine/EditorBlueprintResources/StandardMacros.IsValid` `_玩家角色`
      (:`Is Valid`
        (`Pawn.AddMovementInput` `_玩家角色` (`KismetMathLibrary.GetForwardVector` (`KismetMathLibrary.MakeRotator` 0.0 0.0 (.yaw (`self.GetControlRotation`)))) AxisValue false)))))

(event `InputAxis|MoveRight`
  (params (AxisValue :type "Float (single-precision)"))
  (bind `_玩家角色` (`self.玩家角色`))
  ;[1 1 1] PlayertInput
  ;;[1 1 1] 移动
  (bind _caninput_ (`self.能否进行操作?`))
  (if _caninput_
    (`/Engine/EditorBlueprintResources/StandardMacros.IsValid` `_玩家角色`
      (:`Is Valid`
        (`Pawn.AddMovementInput` `_玩家角色` (`KismetMathLibrary.GetRightVector` (`KismetMathLibrary.MakeRotator` 0.0 0.0 (.yaw (`self.GetControlRotation`)))) AxisValue false)))))

(event `InputAction|IdleState`
  (params (Key :type "Key Structure" :default "AnyKey"))
  (bind `_玩家角色` (`self.玩家角色`))
  ;[1 1 1] PlayertInput
  ;;[1 1 1] 和平/战斗
  (:`Pressed`
    (bind _caninput_ (`self.能否进行操作?`))
    (if _caninput_
      (if (`|EnumEquality` (`/Game/MyGame/MyCharacter/Blueprints/CharacterBP_Action.EqipState` `_玩家角色`) "NewEnumerator2")
        (set `/Game/MyGame/MyCharacter/Blueprints/CharacterBP_Action.EqipState` "NewEnumerator1" `_玩家角色`)
        (else
          (set `/Game/MyGame/MyCharacter/Blueprints/CharacterBP_Action.EqipState` "NewEnumerator2" `_玩家角色`))))))

(event `InputAction|Attack`
  (params (Key :type "Key Structure" :default "AnyKey"))
  (bind `_玩家角色` (`self.玩家角色`))
  ;[1 1 1] PlayertInput
  ;;[1 1 1] 普通攻击
  (:`Pressed`
    (bind _caninput_ (`self.能否进行操作?`))
    (if _caninput_
      (set `/Game/MyGame/MyCharacter/Blueprints/CharacterBP_Action.DoAttack?` true `_玩家角色`)))
  (:`Released`
    (set `/Game/MyGame/MyCharacter/Blueprints/CharacterBP_Action.DoAttack?` false `_玩家角色`)))

(event `InputAction|Block`
  (params (Key :type "Key Structure" :default "AnyKey"))
  (bind `_玩家角色` (`self.玩家角色`))
  ;[1 1 1] PlayertInput
  ;;[1 1 1] 防御
  (:`Pressed`
    (bind _caninput_ (`self.能否进行操作?`))
    (if _caninput_
      (set `/Game/MyGame/MyCharacter/Blueprints/CharacterBP_Action.DoBlock?` true `_玩家角色`)))
  (:`Released`
    (set `/Game/MyGame/MyCharacter/Blueprints/CharacterBP_Action.DoBlock?` false `_玩家角色`)))

(event `InputAction|Jump`
  (params (Key :type "Key Structure" :default "AnyKey"))
  (bind `_玩家角色` (`self.玩家角色`))
  ;[1 1 1] PlayertInput
  ;;[1 1 1] 跳跃
  (:`Pressed`
    (bind _caninput_ (`self.能否进行操作?`))
    (if _caninput_
      (set `/Game/MyGame/MyCharacter/Blueprints/CharacterBP_Action.DoJump?` true `_玩家角色`)))
  (:`Released`
    (set `/Game/MyGame/MyCharacter/Blueprints/CharacterBP_Action.DoJump?` false `_玩家角色`)))

(event `InputAction|Skill0`
  (params (Key :type "Key Structure" :default "AnyKey"))
  (bind `_玩家角色` (`self.玩家角色`))
  ;[1 1 1] PlayertInput
  ;;[1 1 1] 施展技能
  (:`Pressed`
    (bind _caninput_ (`self.能否进行操作?`))
    (if _caninput_
      (set `/Game/MyGame/MyCharacter/Blueprints/CharacterBP_Action.DoSkill` "NewEnumerator1" `_玩家角色`)))
  (:`Released`
    (set `/Game/MyGame/MyCharacter/Blueprints/CharacterBP_Action.DoSkill` "NewEnumerator0" `_玩家角色`)))

(event `InputAction|Interact`
  (params (Key :type "Key Structure" :default "AnyKey"))
  (bind `_互动actor` (`self.互动Actor`))
  (bind `_玩家角色` (`self.玩家角色`))
  ;[1 1 1] PlayertInput
  ;;[1 1 1] 互动
  (:`Released`
    (bind _canaction_ (`self.能否进行互动?`))
    (if _canaction_
      (`|ExecutionSequence`
        (:`then_0`
          (bind _ascharacter_bp_ai (cast `/Game/MyGame/MyCharacter/Blueprints/CharacterBP_AI` `_互动actor`))
          (`self.进行对话` _ascharacter_bp_ai))
        (:`then_1`
          (bind `_as互动物件` (cast `/Game/MyGame/物件/互动物件` `_互动actor`))
          (set `/Game/MyGame/MyCharacter/Blueprints/CharacterBP_Action.EqipState` "NewEnumerator2" `_玩家角色`)
          (`/Game/MyGame/物件/互动物件.与角色互动` `_as互动物件` `_玩家角色`)
          (`self.设置玩家控制器状态` "NewEnumerator3")))
      (elif (`|EnumEquality` (`self.玩家控制器状态`) "NewEnumerator3")
        (bind `_as互动物件_2` (cast `/Game/MyGame/物件/互动物件` `_互动actor`))
        (`/Game/MyGame/物件/互动物件.停止互动` `_as互动物件_2`)
        (`self.设置玩家控制器状态` "NewEnumerator0")))))

(event `InputAxis|Turn`
  (params (AxisValue :type "Float (single-precision)"))
  (bind `_玩家角色` (`self.玩家角色`))
  ;[1 1 1] PlayertInput
  ;;[1 1 1] 视角
  (`/Engine/EditorBlueprintResources/StandardMacros.IsValid` `_玩家角色`
    (:`Is Valid`
      (`Pawn.AddControllerYawInput` `_玩家角色` AxisValue))))

(event `InputAxis|LookUp`
  (params (AxisValue :type "Float (single-precision)"))
  (bind `_玩家角色` (`self.玩家角色`))
  ;[1 1 1] PlayertInput
  ;;[1 1 1] 视角
  (`/Engine/EditorBlueprintResources/StandardMacros.IsValid` `_玩家角色`
    (:`Is Valid`
      (`Pawn.AddControllerPitchInput` `_玩家角色` AxisValue))))

(event `InputAction|Pause`
  (params (Key :type "Key Structure" :default "AnyKey"))
  ;[1 1 1] PlayertInput
  (:`Released`
    (if (`|EnumEquality` (`self.玩家控制器状态`) "NewEnumerator0")
      (`/Game/MyGame/MyGameMode/HUDMessagesFunctionLibrary.SetPauseHUDView` true)
      (`self.设置玩家控制器状态` "NewEnumerator1"))))

(event `Key|LeftBracket`
  (params (Key :type "Key Structure" :default "AnyKey"))
  (:`Released`
    (bind _asmy_game_instance (cast `/Game/MyGame/MyGameMode/MyGameInstance` (`GameplayStatics.GetGameInstance`)))
    (`/Game/MyGame/MyGameMode/MyGameInstance.SaveGame` _asmy_game_instance)))

(event `Key|RightBracket`
  (params (Key :type "Key Structure" :default "AnyKey"))
  (:`Released`
    (bind _asmy_game_instance (cast `/Game/MyGame/MyGameMode/MyGameInstance` (`GameplayStatics.GetGameInstance`)))
    (`/Game/MyGame/MyGameMode/MyGameInstance.LoadGame` _asmy_game_instance)))

(event `Key|K`
  (params (Key :type "Key Structure" :default "AnyKey"))
  (:`Released`
    (bind _savedata (`/Game/MyGame/MyGameMode/GameMessagesFunctionLibrary.GetCurrSaveData`))
    (bind _output_get (set `/Game/MyGame/GameData/MySaveData.GameDateTime` (+ (`/Game/MyGame/GameData/MySaveData.GameDateTime` _savedata) (`KismetMathLibrary.MakeTimespan` 1)) _savedata))
    (`KismetSystemLibrary.PrintString` (`KismetStringLibrary.Conv_IntToString` (`.Day` (`KismetMathLibrary.BreakDateTime` _output_get))))))

(fn `SetDialogue`
  (params (`开关` :type Boolean))
  (bind _dialoguehud (`/Game/MyGame/MyGameMode/HUDMessagesFunctionLibrary.SetDialogueHUDView` `开关`))
  (if `开关`
    (`self.设置玩家控制器状态` "NewEnumerator1")
    (`WidgetBlueprintLibrary.SetInputMode_GameAndUIEx` self _dialoguehud)
    (else
      (`self.设置玩家控制器状态` "NewEnumerator0")))
  (return))

(fn `UserConstructionScript`)

(fn `射线检测互动Actor`
  (bind `_玩家角色` (`self.玩家角色`))
  (bind _returnvalue (`SceneComponent.K2_GetComponentLocation` (`/Game/MyGame/MyCharacter/Blueprints/CharacterBP_Player.SpringArm` `_玩家角色`)))
  (if (`|EnumEquality` (`self.玩家控制器状态`) "NewEnumerator0")
    (bind (_outhit _returnvalue_2) (`KismetSystemLibrary.LineTraceSingle` _returnvalue (+ _returnvalue (* (`SceneComponent.GetForwardVector` (`/Game/MyGame/MyCharacter/Blueprints/CharacterBP_Player.Camera` `_玩家角色`)) 100.0)) "TraceTypeQuery1" false (`|MakeArray` (`GameplayStatics.GetPlayerPawn` 0) :!type "Actor Object Reference")))
    (if _returnvalue_2
      (`|ExecutionSequence`
        (:`then_0`
          (bind (_bblockinghit _binitialoverlap _time _location _impactpoint _normal _impactnormal _physmat _hitactor) (`GameplayStatics.BreakHitResult` _outhit))
          (bind _ascharacter_bp_ai (cast `/Game/MyGame/MyCharacter/Blueprints/CharacterBP_AI` _hitactor)
            (:`then`
              (bind `_输出对象` (`self.是否可与Actor进行对话` _ascharacter_bp_ai)
                (:`成功`
                  (set `self.互动Actor` `_输出对象`)
                  (return))
                (:`失败`
                  _)))
            (:`CastFailed`
              _))
          (set `self.互动Actor` null :!label _label))
        (:`then_1`
          (bind `_as互动物件` (cast `/Game/MyGame/物件/互动物件` _hitactor)
            (:`then`
              (if (== (`/Game/MyGame/物件/互动物件.当前角色` `_as互动物件`) null)
                (set `self.互动Actor` `_as互动物件`)
                (return)))
            (:`CastFailed`
              (goto _label))))
        (:`then_2`
          (return)))
      (else
        (goto _label)))
    (else
      (return))))

(fn `玩家控制器初始化`
  (bind _ascharacter_bp_player (cast `/Game/MyGame/MyCharacter/Blueprints/CharacterBP_Player` (`self.K2_GetPawn`))
    (:`then`
      (set `self.玩家角色` _ascharacter_bp_player))
    (:`CastFailed`
      _))
  (return))

(fn `结束对话`
  (bind _returnvalue (`AIBlueprintHelperLibrary.GetAIController` (`self.互动Actor`)))
  (bind `_asaic_ai控制器` (cast `/Game/MyGame/MyCharacter/Blueprints/AICharacter/AIC_AI控制器` _returnvalue)
    (:`then`
      (`/Game/MyGame/MyCharacter/Blueprints/AICharacter/AIC_AI控制器.SetBlackboardActor` `_asaic_ai控制器` null "对话Actor")
      (`self.SetDialogue` false))
    (:`CastFailed`
      _))
  (return))

(fn `能否进行互动?`
  (returns (`CanAction?` :type Boolean))
  (if (and (!= (`self.互动Actor`) null) (`|EnumEquality` (`self.玩家控制器状态`) "NewEnumerator0"))
    (return true)
    (else
      (return false))))

(fn `能否进行操作?`
  (returns (`CanInput?` :type Boolean))
  (if (`|EnumEquality` (`self.玩家控制器状态`) "NewEnumerator0")
    (return true)
    (else
      (return false))))

(fn `设置玩家控制器状态`
  (params (`玩家状态` :type "/Game/MyGame/MyCharacter/Blueprints/玩家状态Enum Enum"))
  (bind _output_get (set `self.玩家控制器状态` `玩家状态`))
  (switch `/Game/MyGame/MyCharacter/Blueprints/玩家状态Enum` _output_get
    (:`NewEnumerator0`
      (set `self.bShowMouseCursor` false)
      (`WidgetBlueprintLibrary.SetInputMode_GameOnly` self)
      (`/Game/MyGame/MyGameMode/HUDMessagesFunctionLibrary.SetMyHUDView` true)
      (`/Game/MyGame/MyGameMode/HUDMessagesFunctionLibrary.SetInputNoticeHUDView` true))
    (:`NewEnumerator1`
      (set `self.bShowMouseCursor` true)
      (`/Game/MyGame/MyGameMode/HUDMessagesFunctionLibrary.SetInputNoticeHUDView` false)
      (`/Game/MyGame/MyGameMode/HUDMessagesFunctionLibrary.SetMyHUDView` false :!label _label))
    (:`NewEnumerator3`
      (goto _label)))
  (return))

(fn `进行对话`
  (params (`对话目标` :type "/Game/MyGame/MyCharacter/Blueprints/CharacterBP_AI Object Reference"))
  (bind _returnvalue (`AIBlueprintHelperLibrary.GetAIController` `对话目标`))
  (bind `_asaic_ai控制器` (cast `/Game/MyGame/MyCharacter/Blueprints/AICharacter/AIC_AI控制器` _returnvalue)
    (:`then`
      (`/Game/MyGame/MyCharacter/Blueprints/AICharacter/AIC_AI控制器.SetBlackboardActor` `_asaic_ai控制器` (`self.玩家角色`) "对话Actor")
      (`self.SetDialogue` true))
    (:`CastFailed`
      _))
  (return))