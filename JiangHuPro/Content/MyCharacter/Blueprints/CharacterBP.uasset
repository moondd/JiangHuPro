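; Melee combat character with health, mana, modular body and pants meshes on a master pose, and a weapon that sheathes or draws via socket attachment.
; AttackBegin and AttackOver bracket each swing, where right-hand weapon overlaps damage each target once.
; Targets in the blocking state with mana negate hits from the front, playing a block montage; others take damage and a hit effect.
; Attacking and blocking can cost mana; zero health flags death.
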(event `self.ReceiveBeginPlay`
  (bind _ascharacter_anim (cast `/Game/MyCharacter/Animations/CharacterAnim` (`SkeletalMeshComponent.GetAnimInstance` (`self.Mesh`))))
  (set `self.CharacterAnim` _ascharacter_anim))

(event `self.ReceiveTick`
  (params (DeltaSeconds :type "Float (single-precision)"))
  (bind _weapontrail (`self.WeaponTrail`))
  ;[1 1 1] WeaponsTrail
  (if (`|EnumEquality` (`self.CharacterState`) "NewEnumerator1")
    (`ActorComponent.SetActive` _weapontrail true false)
    (else
      (`ActorComponent.SetActive` _weapontrail false false))))

(event `self.R-Hand.OnComponentBeginOverlap`
  (params (OverlappedComponent :type "PrimitiveComponent Object Reference") (OtherActor :type "Actor Object Reference") (OtherComp :type "PrimitiveComponent Object Reference") (OtherBodyIndex :type Integer) (bFromSweep :type Boolean) (SweepResult :type "HitResult Structure (by ref)"))
  (bind _returnvalue (`self.K2_GetActorLocation` OtherActor))
  (bind _r_hand (`self.R-Hand`))
  (bind _returnvalue_2 (`SceneComponent.GetSocketLocation` _r_hand "EffectStart"))
  ;[1 1 1] 伤害
  (bind (_returncandamage _damagestate) (`self.CanDamage` OtherActor))
  (if _returncandamage
    (bind _isblocking_ (`self.TargetIsBlocking` OtherActor _damagestate))
    (if (not _isblocking_)
      (`GameplayStatics.SpawnEmitterAttached` "/Game/MyEffects/BeDamage_Normal.BeDamage_Normal" OtherComp "None" (- _returnvalue_2 (* (- _returnvalue_2 _returnvalue) 0.5)) (`KismetMathLibrary.MakeRotator` (+ (.roll (`SceneComponent.GetSocketRotation` _r_hand "EffectStart")) 90.0) (.pitch (`KismetMathLibrary.FindLookAtRotation` (`self.K2_GetActorLocation`) _returnvalue)) (.yaw (`KismetMathLibrary.FindLookAtRotation` (`self.K2_GetActorLocation`) _returnvalue))) "KeepWorldPosition")
      (`GameplayStatics.ApplyDamage` OtherActor 25.0))))

(event `self.ReceiveAnyDamage`
  (params (Damage :type "Float (single-precision)") (DamageType :type "DamageType Object Reference") (InstigatedBy :type "Controller Object Reference") (DamageCauser :type "Actor Object Reference"))
  (bind _currhealth (`self.CurrHealth`))
  (set `self.CurrHealth` (- _currhealth Damage))
  (if (<= _currhealth 0.0)
    (set `self.IsDeath?` true)
    (`PrimitiveComponent.SetCollisionEnabled` (`self.CapsuleComponent`) "NoCollision")))

(fn `AttackBegin`
  (params (NewParam :type "/Game/MyCharacter/Animations/Enum_DamageState Enum"))
  (bind _output_get (set `self.DamageState` NewParam))
  (bind _needmanatodamage (`self.NeedManaToDamage` _output_get))
  (`self.SetCurrMana` _needmanatodamage))

(fn `AttackOver`
  (set `self.DamageState` "NewEnumerator4")
  (`KismetArrayLibrary.Array_Clear` (`self.AttackTargets`)))

(fn `BeDamage`
  (params (DamageState :type "/Game/MyCharacter/Animations/Enum_DamageState Enum"))
  (set `/Game/MyCharacter/Animations/CharacterAnim.BeDamageState` DamageState (`self.CharacterAnim`)))

(fn `CanDamage`
  (params (OtherActor :type "Actor Object Reference"))
  (returns (ReturnCanDamage :type Boolean) (DamageState :type "/Game/MyCharacter/Animations/Enum_DamageState Enum"))
  (bind _attacktargets (`self.AttackTargets`))
  (if (`|EnumInequality` (`self.DamageState`) "NewEnumerator4")
    (if (!= OtherActor self)
      (if (`KismetArrayLibrary.Array_Contains` _attacktargets OtherActor)
        _
        (else
          (`KismetArrayLibrary.Array_Add` _attacktargets OtherActor)
          (return true (`self.DamageState`))))))
  (return false "NewEnumerator4"))

(fn `DamageIsBlocking`
  (params (DamageState :type "/Game/MyCharacter/Animations/Enum_DamageState Enum"))
  (bind _needmanatodamage (`self.NeedManaToDamage` DamageState))
  (`self.SetCurrMana` _needmanatodamage)
  (`self.PlayAnimMontage` self "/Game/MyCharacter/Animations/Montage/Block.Block" 0.6 "Blockinig"))

(fn `NeedManaToDamage`
  (params (DamageState :type "/Game/MyCharacter/Animations/Enum_DamageState Enum"))
  (returns (NeedManaToDamage :type "Float (double-precision)"))
  (`|ExecutionSequence`
    (:`then_0`
      (if (`|EnumEquality` DamageState "NewEnumerator0")
        (return -20.0)))))

(fn `SetCurrMana`
  (params (Value :type "Float (double-precision)"))
  (set `self.CurrMana` (+ (`self.CurrMana`) Value)))

(fn `SetEqip`
  (bind _weapontrail (`self.WeaponTrail`))
  (`SceneComponent.K2_AttachTo` (`self.R-Hand`) (`self.Mesh`) "Bip001-R-Hand-Socket" "SnapToTargetIncludingScale" true)
  (set `self.IsREqip?` true)
  (`SceneComponent.K2_AttachTo` _weapontrail (`self.R-Hand`) "None" "SnapToTargetIncludingScale" true)
  (`ParticleSystemComponent.BeginTrails` _weapontrail "EffectStart" "EffectOver" "ETrailWidthMode_FromFirst" 1.0))

(fn `SetMesh`
  (`|ExecutionSequence`
    (:`then_0`
      (bind _output_get (set `self.Body` (`self.Body`)))
      (`SkinnedMeshComponent.SetSkinnedAssetAndUpdate` _output_get (`self.BodyMesh`) false))
    (:`then_1`
      (bind _output_get_2 (set `self.Pants` (`self.Pants`)))
      (`SkinnedMeshComponent.SetSkinnedAssetAndUpdate` _output_get_2 (`self.PantsMesh`) false))))

(fn `SetSkillsStruct`
  (params (SkillID :type Integer))
  (bind _returnvalue (`|GetDataTableRow` "/Game/MyCharacter/SkillsDataTable.SkillsDataTable" "1")
    (:`then`
      (set `self.SkillsStruct` (`|MakeArray` _returnvalue _returnvalue (struct) (struct) (struct) (struct))))))

(fn `SetUnEquip`
  (`SceneComponent.K2_AttachTo` (`self.R-Hand`) (`self.L_Hand`) "Socket" "SnapToTargetIncludingScale" true)
  (set `self.IsREqip?` false)
  (set `self.IsLEqip?` true))

(fn `TargetIsBlocking`
  (params (TargetActor :type "Actor Object Reference") (DamageState :type "/Game/MyCharacter/Animations/Enum_DamageState Enum"))
  (returns (`IsBlocking?` :type Boolean))
  (bind _ascharacter_bp (cast `/Game/MyCharacter/Blueprints/CharacterBP` TargetActor)
    (:`then`
      (if (and (> (`/Game/MyCharacter/Blueprints/CharacterBP.CurrMana` _ascharacter_bp) 0.0) (`|EnumEquality` (`/Game/MyCharacter/Blueprints/CharacterBP.CharacterState` _ascharacter_bp) "NewEnumerator2") (< (`KismetMathLibrary.DegAcos` (`KismetMathLibrary.Dot_VectorVector` (`KismetMathLibrary.Normal` (- (`self.K2_GetActorLocation` self) (`self.K2_GetActorLocation` TargetActor))) (`self.GetActorForwardVector` TargetActor))) 90.0))
        (`self.DamageIsBlocking` _ascharacter_bp DamageState)
        (return true)
        (else
          (`self.BeDamage` _ascharacter_bp DamageState))))
    (:`CastFailed`
      _))
  (return false))

(fn `UserConstructionScript`
  (bind _mesh (`self.Mesh`))
  (`SkinnedMeshComponent.SetLeaderPoseComponent` (`self.Body`) _mesh)
  (`SkinnedMeshComponent.SetLeaderPoseComponent` (`self.Pants`) _mesh)
  (`self.SetUnEquip`)
  (`self.SetSkillsStruct` 0))