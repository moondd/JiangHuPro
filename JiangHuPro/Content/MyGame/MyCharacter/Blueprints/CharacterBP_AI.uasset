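; AI character Blueprint that derives its interaction state and dialogue ID from its relationship and alignment (性向) relative to the player.
; On BeginPlay it caches the player character and updates the interaction state.
; Strangers get a fixed state; normal relationships switch state when evil AI meets a neutral-or-good player or good AI an evil one.
; Dialogue ID lookup uses the relationship name for strangers, otherwise the AI's identity unless alignments clash.
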(event `self.ReceiveBeginPlay`
  (`parent.ReceiveBeginPlay`)
  (bind _ascharacter_bp_player (cast `/Game/MyGame/MyCharacter/Blueprints/CharacterBP_Player` (`GameplayStatics.GetPlayerPawn` 0)))
  (set `self.玩家角色` _ascharacter_bp_player)
  (`self.更新AI与玩家互动关系`))

(event `self.ReceiveTick`
  (params (DeltaSeconds :type "Float (single-precision)"))
  (`parent.ReceiveTick` 0.0))

(fn `UserConstructionScript`
  (`parent.UserConstructionScript`))

(fn `更新AI与玩家互动关系`
  (bind _returnvalue (`KismetMathLibrary.Conv_ByteToInt` (`/Game/MyGame/MyCharacter/Blueprints/MyCharacterBP.性向` (`self.玩家角色`))))
  (switch `/Game/MyGame/MyCharacter/Blueprints/特殊关系Enum` (`self.AI与玩家特殊关系`)
    (:`NewEnumerator1`
      (set `self.AI互动状态` "NewEnumerator0"))
    (:`NewEnumerator0`
      (switch `/Game/MyGame/MyCharacter/Blueprints/性向Enum` (`self.性向`)
        (:`NewEnumerator0`
          (if (> _returnvalue 1) :!label _label
            (set `self.AI互动状态` "NewEnumerator1" :!label _label_2)))
        (:`NewEnumerator1`
          (goto _label))
        (:`NewEnumerator2`
          _)
        (:`NewEnumerator3`
          (if (< _returnvalue 2) :!label _label_3
            (goto _label_2)
            (else
              _)))
        (:`NewEnumerator4`
          (goto _label_3)))))
  (return))

(fn `获取当前对话ID`
  (bind _returnvalue (`KismetMathLibrary.Conv_ByteToInt` (`/Game/MyGame/MyCharacter/Blueprints/MyCharacterBP.性向` (`self.玩家角色`))))
  (switch `/Game/MyGame/MyCharacter/Blueprints/特殊关系Enum` (`self.AI与玩家特殊关系`)
    (:`NewEnumerator1`
      (set `self.当前对话ID` (`KismetStringLibrary.Conv_StringToName` (`|GetEnumeratorNameAsString` (`self.AI与玩家特殊关系`))))
      (return))
    (:`NewEnumerator0`
      (switch `/Game/MyGame/MyCharacter/Blueprints/性向Enum` (`self.性向`)
        (:`NewEnumerator0`
          (if (> _returnvalue 1) :!label _label
            _
            (else
              (set `self.当前对话ID` (`self.身份`) :!label _label_2)
              (return))))
        (:`NewEnumerator1`
          (goto _label))
        (:`NewEnumerator2`
          (goto _label_2))
        (:`NewEnumerator3`
          (if (< _returnvalue 2) :!label _label_3
            (return)
            (else
              (goto _label_2))))
        (:`NewEnumerator4`
          (goto _label_3)))
      (return))))